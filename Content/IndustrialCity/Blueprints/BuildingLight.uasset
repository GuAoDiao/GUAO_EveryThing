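; BuildingLight is an Industrial City prop that pairs a static mesh with a point light as a configurable building light.
; All logic runs in the Construction Script, which applies the shadow and intensity settings to the light.
; A toggle shows or hides the light and drives the mesh's emissive strength through a dynamic material instance, scaled from light intensity or zeroed when off.
; The event graph is unused.
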(event EventBeginPlay)

(event EventActorBeginOverlap
  (params (OtherActor :type Actor%20Object%20Reference)))

(event EventTick
  (params (DeltaSeconds :type Float%20%28single-precision%29)))

(fn ConstructionScript
  (bind _light_intensity (Variables|Default|GetLight_Intensity))
  (bind _pointlight (Variables|Default|GetPointLight))
  (bind _returnvalue (Rendering|Material|CreateDynamicMaterialInstance (Variables|Default|GetStaticMesh) 0 "/Game/IndustrialCity/Materials/BuildingLight.BuildingLight" :!class /Script/Engine.PrimitiveComponent))
  (LocalVariables|SetDMI _returnvalue)
  (Rendering|Components|Light|SetCastShadows _pointlight (Variables|Default|GetCastShadows))
  (Rendering|Components|Light|SetIntensity _pointlight _light_intensity)
  (if (Variables|Default|GetLightToggle)
    (Rendering|Material|SetScalarParameterValue (LocalVariables|GetDMI) "Emissive Strength" (/ _light_intensity 1e+03) :!class /Script/Engine.MaterialInstanceDynamic)
    (Rendering|SetVisibility _pointlight true false)
    (else
      (Rendering|Material|SetScalarParameterValue (LocalVariables|GetDMI) "Emissive Strength" 0.0 :!class /Script/Engine.MaterialInstanceDynamic)
      (Rendering|SetVisibility _pointlight false false))))