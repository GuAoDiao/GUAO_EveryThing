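; BP_Road is a configurable road piece for the Industrial City environment, with two-lane and four-lane sizes.
; The construction script switches on road size, curb variation, sidewalk variation and a sidewalk depth flag (wide or short) to select the matching pre-placed components.
; It toggles the visibility of each selection rather than setting it explicitly, so the result depends on each component's default visibility.
; The event graph has no runtime logic.
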(event `self.ReceiveBeginPlay`)

(event `self.ReceiveActorBeginOverlap`
  (params (OtherActor :type "Actor Object Reference")))

(event `self.ReceiveTick`
  (params (DeltaSeconds :type "Float (single-precision)")))

(fn `UserConstructionScript`
  (bind _sidewalkdepth (`self.SidewalkDepth`))
  (bind _sidewalkdepth_2 (`self.SidewalkDepth`))
  (switch `/Game/IndustrialCity/Blueprints/PP_Roads` (`self.Road Size`)
    (:`NewEnumerator0`
      (`SceneComponent.ToggleVisibility` (`self.Road_2L`) false)
      (switch `/Game/IndustrialCity/Blueprints/PP_Curbs` (`self.Curb_Variation`)
        (:`NewEnumerator0`
          (`SceneComponent.ToggleVisibility` (`self.Curb_2L_VarA`) false))
        (:`NewEnumerator1`
          (`SceneComponent.ToggleVisibility` (`self.Curb_2L_VarB`) false))
        (:`NewEnumerator2`
          (`SceneComponent.ToggleVisibility` (`self.Curb_2L_VarC`) false))
        (:`NewEnumerator3`
          (`SceneComponent.ToggleVisibility` (`self.Curb_2L_VarD`) false)))
      (switch `/Game/IndustrialCity/Blueprints/PP_Sidewalks` (`self.Sidewalk Variation`)
        (:`NewEnumerator0`
          (if _sidewalkdepth_2
            (`SceneComponent.ToggleVisibility` (`self.Sidewalk_2L_VarA_Wide`) false)
            (else
              (`SceneComponent.ToggleVisibility` (`self.Sidewalk_2L_VarA_Short`) false))))
        (:`NewEnumerator1`
          (if _sidewalkdepth_2
            (`SceneComponent.ToggleVisibility` (`self.Sidewalk_2L_VarB_Wide`) false)
            (else
              (`SceneComponent.ToggleVisibility` (`self.Sidewalk_2L_VarB_Short`) false))))
        (:`NewEnumerator2`
          (if _sidewalkdepth_2
            (`SceneComponent.ToggleVisibility` (`self.Sidewalk_2L_VarC_Wide`) false)
            (else
              (`SceneComponent.ToggleVisibility` (`self.Sidewalk_2L_VarC_Short`) false))))
        (:`NewEnumerator3`
          (if _sidewalkdepth_2
            (`SceneComponent.ToggleVisibility` (`self.Sidewalk_2L_VarD_Wide`) false)
            (else
              (`SceneComponent.ToggleVisibility` (`self.Sidewalk_2L_VarD_Short`) false))))))
    (:`NewEnumerator1`
      (`SceneComponent.ToggleVisibility` (`self.Road_4L`) false)
      (switch `/Game/IndustrialCity/Blueprints/PP_Curbs` (`self.Curb_Variation`)
        (:`NewEnumerator0`
          (`SceneComponent.ToggleVisibility` (`self.Curb_4L_VarA`) false))
        (:`NewEnumerator1`
          (`SceneComponent.ToggleVisibility` (`self.Curb_4L_VarB`) false))
        (:`NewEnumerator2`
          (`SceneComponent.ToggleVisibility` (`self.Curb_4L_VarC`) false))
        (:`NewEnumerator3`
          (`SceneComponent.ToggleVisibility` (`self.Curb_4L_VarD`) false)))
      (switch `/Game/IndustrialCity/Blueprints/PP_Sidewalks` (`self.Sidewalk Variation`)
        (:`NewEnumerator0`
          (if _sidewalkdepth
            (`SceneComponent.ToggleVisibility` (`self.Sidewalk_4L_VarA_Wide`) false)
            (else
              (`SceneComponent.ToggleVisibility` (`self.Sidewalk_4L_VarA_Short`) false))))
        (:`NewEnumerator1`
          (if _sidewalkdepth
            (`SceneComponent.ToggleVisibility` (`self.Sidewalk_4L_VarB_Wide`) false)
            (else
              (`SceneComponent.ToggleVisibility` (`self.Sidewalk_4L_VarB_Short`) false))))
        (:`NewEnumerator2`
          (if _sidewalkdepth
            (`SceneComponent.ToggleVisibility` (`self.Sidewalk_4L_VarC_Wide`) false)
            (else
              (`SceneComponent.ToggleVisibility` (`self.Sidewalk_4L_VarC_Short`) false))))
        (:`NewEnumerator3`
          (if _sidewalkdepth
            (`SceneComponent.ToggleVisibility` (`self.Sidewalk_4L_VarD_Wide`) false)
            (else
              (`SceneComponent.ToggleVisibility` (`self.Sidewalk_4L_VarD_Short`) false))))))))